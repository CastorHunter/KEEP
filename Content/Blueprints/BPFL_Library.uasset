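; BPFL_Library is a Blueprint function library with shortcuts to the first player's core objects.
; GetPlayer and GetController return the index 0 pawn and controller, cast to BP_Player and BP_PlayerController.
; GetOnMobile builds on GetController to expose the controller's OnMobile value.
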(fn `GetController`
  (returns (PlayerController :type "/Game/Blueprints/Player/BP_PlayerController Object Reference"))
  (bind _asbp_player_controller (cast `/Game/Blueprints/Player/BP_PlayerController` (`GameplayStatics.GetPlayerController` null)))
  (return _asbp_player_controller))

(fn `GetOnMobile`
  (returns (OnMobile :type Boolean))
  (return (`/Game/Blueprints/Player/BP_PlayerController.OnMobile` (`self.GetController` null))))

(fn `GetPlayer`
  (returns (Player :type "/Game/Blueprints/Player/BP_Player Object Reference"))
  (bind _asbp_player (cast `/Game/Blueprints/Player/BP_Player` (`GameplayStatics.GetPlayerPawn` null)))
  (return _asbp_player))