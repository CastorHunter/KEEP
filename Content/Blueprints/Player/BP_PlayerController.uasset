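; Player controller for a stealth game with closet hiding, handling input, cursor locking, UI creation, noise making and death by reloading the level.
; Camera line traces highlight the current BP_Interactable for Interact, while mouse clicks also feed the QTE manager.
; Sprint drives a delay-looped stamina meter, HearSound uses a timeline for a prioritized sound-sensor display, and a stress timeline forces closet exit.
; BeginPlay currently forces OnMobile true for testing, leaving platform detection disconnected.
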(event `HearSound`
  (params (SoundToHear :type "/Game/Enums/E_SoundLoudness Enum" :default "NewEnumerator0") (SoundDuration :type "Float (double-precision)" :default 0.7))
  (bind _soundvolume (`self.SoundVolume`))
  ; Sound Sensor Update System
  (`TimelineComponent.SetTimelineLength` (`self.SoundDuration`) SoundDuration)
  (if (`|EnumEquality` SoundToHear "NewEnumerator0")
    (bind _output_get (set `self.SoundVolume` "NewEnumerator0"))
    (`/Game/Blueprints/UI/WBP_PlayerUI.UpdateSoundSensor` (`self.PlayerUI`) _output_get)
    (`Timeline|SoundDuration` :!via `PlayFromStart` :!label _label
      (:`Finished`
        (bind _output_get_2 (set `self.SoundVolume` "NewEnumerator3"))
        (`/Game/Blueprints/UI/WBP_PlayerUI.UpdateSoundSensor` (`self.PlayerUI`) _output_get_2)))
    (elif (`|EnumEquality` SoundToHear "NewEnumerator1")
      (bind _output_get_3 (set `self.SoundVolume` "NewEnumerator1"))
      (`/Game/Blueprints/UI/WBP_PlayerUI.UpdateSoundSensor` (`self.PlayerUI`) _output_get_3)
      (goto _label :!via `PlayFromStart`)
      (elif (`|EnumEquality` (`self.SoundVolume`) "NewEnumerator0")
        (`self.HearSound` "NewEnumerator1" (- SoundDuration (`TimelineComponent.GetPlaybackPosition` (`self.SoundDuration`))))
        (elif (`|EnumEquality` SoundToHear "NewEnumerator2")
          (bind _output_get_4 (set `self.SoundVolume` "NewEnumerator2"))
          (`/Game/Blueprints/UI/WBP_PlayerUI.UpdateSoundSensor` (`self.PlayerUI`) _output_get_4)
          (goto _label :!via `PlayFromStart`)
          (elif (or (`|EnumEquality` _soundvolume "NewEnumerator0") (`|EnumEquality` _soundvolume "NewEnumerator1"))
            (`self.HearSound` "NewEnumerator2" (- SoundDuration (`TimelineComponent.GetPlaybackPosition` (`self.SoundDuration`))))))))))

(event `HideMouse`
  (bind _playercontroller (`/Game/Blueprints/BPFL_Library.GetController`))
  ; Hide and Show Mouse Cursor while locking and unlocking it
  (if (not (`self.OnMobile`))
    (`self.SetIgnoreLookInput` _playercontroller false)
    (set `PlayerController.bShowMouseCursor` false _playercontroller)
    (`WidgetBlueprintLibrary.SetFocusToGameViewport`)
    (`GameplayStatics.SetViewportMouseCaptureMode` "CapturePermanently")))

(event `EnhancedInput|/Game/Inputs/IA_Aim`
  (params (ActionValue :type "Vector2D Structure") (ElapsedSeconds :type "Float (double-precision)") (TriggeredSeconds :type "Float (double-precision)") (InputAction :type "InputAction Object Reference" :default "/Game/Inputs/IA_Aim.IA_Aim"))
  ; Inputs
  (:`Triggered`
    (`/Game/Blueprints/Player/BP_Player.Aim` (`/Game/Blueprints/BPFL_Library.GetPlayer`) ActionValue_X ActionValue_Y)))

(event `ShowMouse`
  (bind _playercontroller (`/Game/Blueprints/BPFL_Library.GetController`))
  ; Hide and Show Mouse Cursor while locking and unlocking it
  (if (not (`self.OnMobile`))
    (set `PlayerController.bShowMouseCursor` true _playercontroller)
    (`GameplayStatics.SetViewportMouseCaptureMode` "NoCapture")
    (`self.SetIgnoreLookInput` _playercontroller true)))

(event `EnhancedInput|/Game/Inputs/IA_Move`
  (params (ActionValue :type "Vector2D Structure") (ElapsedSeconds :type "Float (double-precision)") (TriggeredSeconds :type "Float (double-precision)") (InputAction :type "InputAction Object Reference" :default "/Game/Inputs/IA_Move.IA_Move"))
  (bind _player (`/Game/Blueprints/BPFL_Library.GetPlayer`))
  (bind _charactermovement (`Character.CharacterMovement` _player))
  ; Inputs
  (:`Triggered`
    (`/Game/Blueprints/Player/BP_Player.Move` _player ActionValue_X ActionValue_Y))
  (:`Started`
    (set `CharacterMovementComponent.bOrientRotationToMovement` false _charactermovement))
  (:`Canceled`
    (set `CharacterMovementComponent.bOrientRotationToMovement` true _charactermovement :!label _label_2))
  (:`Completed`
    (goto _label_2)))

(event `StartStressing`
  (bind _stress (`self.Stress`))
  (bind _wbp_closetui (`/Game/Blueprints/UI/WBP_MainUI.WBP_ClosetUI` (`self.MainUI`)))
  ; Force leaving closet when stress is too high
  (set `self.Stress` 0.0)
  (`Timeline|StressTimeline` :`NewTime` 1000.0 :!via `PlayFromStart` :!label _label_3
    (:`Update`
      (set `self.Stress` (+ _stress 1.0))
      (`/Game/Blueprints/UI/WBP_ClosetUI.UpdateStressBar` _wbp_closetui)
      (if (== _stress (`self.MaxStress`))
        (`/Game/Blueprints/UI/WBP_ClosetUI.LeaveCloset` _wbp_closetui)
        (goto _label_3 :!via `Stop`)))))

(event `EnhancedInput|/Game/Inputs/IA_Sprint`
  (params (ActionValue :type Boolean) (ElapsedSeconds :type "Float (double-precision)") (TriggeredSeconds :type "Float (double-precision)") (InputAction :type "InputAction Object Reference" :default "/Game/Inputs/IA_Sprint.IA_Sprint"))
  ; Inputs
  (:`Started`
    (`self.Sprint`))
  (:`Canceled`
    (`self.StopSprinting` :!label _label_4))
  (:`Completed`
    (goto _label_4)))

(event `StopSprinting`
  (bind _returnvalue (not (`self.Running`)))
  ; Sprint
  (set `CharacterMovementComponent.MaxWalkSpeed` (`self.WalkSpeed`) (`Character.CharacterMovement` (`/Game/Blueprints/BPFL_Library.GetPlayer`)) :!label _label_5)
  (set `self.Running` false)
  ;; Handles Stamina
  (if (not (and (== (`self.MaxStamina`) (`self.Stamina`)) _returnvalue)) :!label _label_6
    (set `self.Stamina` (`KismetMathLibrary.FClamp` (+ (`self.Stamina`) (- (* (`KismetMathLibrary.Conv_BoolToDouble` _returnvalue) 2.0) 1.5)) 0.0 (`self.MaxStamina`)))
    (`KismetSystemLibrary.Delay` 0.01)
    (`/Game/Blueprints/UI/WBP_PlayerUI.UpdateStamina` (`self.PlayerUI`))
    (if (== (`self.Stamina`) 0.0)
      (goto _label_5)
      (else
        (goto _label_6)))))

(event `Sprint`
  ; Sprint
  (set `CharacterMovementComponent.MaxWalkSpeed` (`self.RunSpeed`) (`Character.CharacterMovement` (`/Game/Blueprints/BPFL_Library.GetPlayer`)))
  (set `self.Running` true)
  (goto _label_6))

(event `CheckIfInteract`
  (bind _player (`/Game/Blueprints/BPFL_Library.GetPlayer`))
  (bind _currentinteractable (`self.CurrentInteractable`))
  (bind _currentinteractable_2 (`self.CurrentInteractable`))
  ; Trace a ray to show off and get interactables
  (bind _returnvalue (`BlueprintCameraPoseFunctionLibrary.MakeCameraPoseFromCameraComponent` (`/Game/Blueprints/Player/BP_Player.Camera` _player)))
  (bind (_origin _direction) (break `Ray` (`BlueprintCameraPoseFunctionLibrary.GetAimRay` _returnvalue)))
  (bind _outhit (`KismetSystemLibrary.LineTraceSingle` _origin (+ _origin (* _direction 250.0)) "TraceTypeQuery2" false (`|MakeArray` _player :!type "Actor Object Reference")))
  (bind (_asbp_interactable _bsuccess) (cast `/Game/Blueprints/Interactables/BP_Interactable` (`.HitActor` (`GameplayStatics.BreakHitResult` _outhit)) :!pure true))
  (if _bsuccess
    (if (`/Game/Blueprints/Interactables/BP_Interactable.Interactable` _asbp_interactable)
      (`/Engine/EditorBlueprintResources/StandardMacros.IsValid` _currentinteractable_2
        (:`Is Valid`
          (if (!= _asbp_interactable _currentinteractable_2)
            (`/Game/Blueprints/Interactables/BP_Interactable.HideInteractable` (`self.CurrentInteractable`))))
        (:`Is Not Valid`
          _))
      (bind _output_get (set `self.CurrentInteractable` _asbp_interactable))
      (`/Game/Blueprints/Interactables/BP_Interactable.ShowInteractable` _output_get)
      (if (`self.OnMobile`)
        (`Widget.SetVisibility` (`/Game/Blueprints/UI/WBP_PlayerUI.InteractButton` (`self.PlayerUI`)) "Visible")))
    (else
      (`/Engine/EditorBlueprintResources/StandardMacros.IsValid` _currentinteractable
        (:`Is Valid`
          (`/Game/Blueprints/Interactables/BP_Interactable.HideInteractable` _currentinteractable)
          (set `self.CurrentInteractable` null)
          (if (`self.OnMobile`)
            (`Widget.SetVisibility` (`/Game/Blueprints/UI/WBP_PlayerUI.InteractButton` (`self.PlayerUI`)) "Hidden")))))))

(event `Key|G`
  (params (Key :type "Key Structure"))
  ;[0.5855 0.5183 0 0.5] G for debug, escape for build
  (:`Pressed`
    (`/Game/Blueprints/UI/WBP_MainUI.TriggerOptionsMenu` (`self.MainUI`))))

(event `Key|LeftMouseButton`
  (params (Key :type "Key Structure"))
  (bind _qtemanager (`self.QTEManager`))
  ; Interact with left mouse click
  (:`Pressed`
    (`/Game/Blueprints/BP_QTE_Manager.Set Pressed Position` _qtemanager)
    (`self.Interact`))
  (:`Released`
    (`/Game/Blueprints/BP_QTE_Manager.Set Released Position` _qtemanager)))

(event `InputTouch` :consume false
  (params (Location :type "Vector Structure") (FingerIndex :type "ETouchIndex Enum"))
  ; Interact with mobile touch
)

(event `self.ReceiveBeginPlay`
  (bind _wbp_qteui (`/Game/Blueprints/UI/WBP_MainUI.WBP_QTEUI` (`self.MainUI`)))
  (`|ExecutionSequence`
    (:`then_0`
      ;[0.2424 0.5972 0.8594 0.5] testing
      (set `self.OnMobile` true))
    (:`then_1`
      (`EnhancedInputSubsystemInterface.AddMappingContext` (subsystem `EnhancedInputLocalPlayerSubsystem`) "/Game/Inputs/IMC_MouseLook.IMC_MouseLook" 0 (struct)))
    (:`then_2`
      (if (`self.IsLocalPlayerController`)
        (`EnhancedInputSubsystemInterface.AddMappingContext` (subsystem `EnhancedInputLocalPlayerSubsystem`) "/Game/Inputs/IMC_Default.IMC_Default" 0 (struct))
        (set `CharacterMovementComponent.MaxWalkSpeed` (`self.WalkSpeed`) (`Character.CharacterMovement` (`/Game/Blueprints/BPFL_Library.GetPlayer`)))
        (set `self.Stamina` (`self.MaxStamina`))
        (bind _returnvalue (`|CreateWidget` "/Game/Blueprints/UI/WBP_MainUI.WBP_MainUI_C"))
        (set `self.MainUI` _returnvalue)
        (set `self.PlayerUI` (`/Game/Blueprints/UI/WBP_MainUI.WBP_PlayerUI` _returnvalue))
        (`UserWidget.AddToViewport` _returnvalue 0)
        (`/Game/Blueprints/UI/WBP_PlayerUI.UpdateStamina` (`self.PlayerUI`))
        (`KismetSystemLibrary.K2_SetTimerDelegate` (`|CreateDelegate` :!event `CheckIfInteract`) 0.2 true)
        (`KismetSystemLibrary.Delay` 0.2)
        (set `/Game/Blueprints/UI/WBP_QTEUI.QTEManager` (`self.QTEManager`) _wbp_qteui)
        (set `self.QTEUI` _wbp_qteui)))
    (:`then_3`
      (`self.HideMouse`))))

(fn `Interact`
  (bind _currentinteractable (`self.CurrentInteractable`))
  (if (not (`/Game/Blueprints/Player/BP_Player.Frozen` (`/Game/Blueprints/BPFL_Library.GetPlayer`)))
    (`/Engine/EditorBlueprintResources/StandardMacros.IsValid` _currentinteractable
      (:`Is Valid`
        (`/Game/Blueprints/Interactables/BP_Interactable.Interact` _currentinteractable)))))

(fn `KillPlayer`
  (`GameplayStatics.OpenLevelBySoftObjectPtr` "/Game/Levels/L_GameLevel.L_GameLevel"))

(fn `MakeASound`
  (params (`Sound Loudness` :type "/Game/Enums/E_SoundLoudness Enum" :default "NewEnumerator0") (SoundToPlay :type "SoundBase Object Reference"))
  (locals (SoundLoudness :type "Map of /Game/Enums/E_SoundLoudness Enum to Float (double-precision)"))
  (bind _player (`/Game/Blueprints/BPFL_Library.GetPlayer`))
  (`self.MakeNoise` _player (`BlueprintMapLibrary.Map_Find` (`local.SoundLoudness`) `Sound Loudness`) _player (`self.K2_GetActorLocation` _player) 1.0 "None")
  (`GameplayStatics.PlaySoundAtLocation` SoundToPlay (`self.K2_GetActorLocation` (`/Game/Blueprints/BPFL_Library.GetPlayer`)) (struct) 1.0 1.0 0.0 null null null null))

(fn `UserConstructionScript`)