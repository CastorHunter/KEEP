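; Touch-controlled player Blueprint with camera look, freezable movement, hiding and an item inspection mode.
; Touch drags that start on the screen's right half steer the camera, while Move and Aim apply axis input unless frozen.
; Inspection spawns BP_InspectItem on nested yaw/pitch pivots, currently always showing a key mesh, and blocks move/look input.
; Dragging the item rotates it with clamped pitch; touching elsewhere exits.
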(event `self.ReceiveBeginPlay`
  (set `self.HUD Ref` (`/Game/Blueprints/Player/BP_PlayerController.PlayerUI` (`/Game/Blueprints/BPFL_Library.GetController`))))

(event `Key|E`
  (params (Key :type "Key Structure"))
  (:`Pressed`
    (`KismetSystemLibrary.PrintString` (`KismetStringLibrary.Conv_IntToString` (/ (`PlayerController.GetViewportSize` (`/Game/Blueprints/BPFL_Library.GetController`)) 2)))))

(event `InputTouch`
  (params (Location :type "Vector Structure") (FingerIndex :type "ETouchIndex Enum"))
  (bind _returnvalue (`KismetMathLibrary.MakeVector2D` Location_X Location_Y))
  (bind _returnvalue_2 (`KismetMathLibrary.MakeVector2D` Location_X Location_Y))
  (bind (_hitresult _returnvalue_3) (`PlayerController.GetHitResultUnderFingerByChannel` (`GameplayStatics.GetPlayerController` 0) "Touch1" "TraceTypeQuery1" true))
  (bind (_x _y) (`KismetMathLibrary.BreakVector2D` (- _returnvalue_2 (`self.LastTouchPos`))))
  (:`Pressed`
    (`KismetSystemLibrary.PrintString` "Pressed")
    (if (`self.IsInspecting`)
      (if _returnvalue_3
        (if (== (`.HitActor` (`GameplayStatics.BreakHitResult` _hitresult)) (`self.InspectActor`))
          (set `self.IsRotatingInspect` true)
          (set `self.LastTouchPos` (`KismetMathLibrary.MakeVector2D` Location_X Location_Y))
          (else
            (`self.StopInspectItem`)))
        (else
          (`self.StopInspectItem`)))
      (elif (> (`KismetMathLibrary.FTrunc` Location_X) (/ (`PlayerController.GetViewportSize` (`/Game/Blueprints/BPFL_Library.GetController`)) 2))
        (set `self.IsRightSide` true)
        (set `self.TouchStartLocation` _returnvalue))))
  (:`Released`
    (if (not (`self.IsRotatingInspect`))
      (set `self.IsRightSide` true)))
  (:`Moved`
    (`KismetSystemLibrary.PrintString` "moved")
    (if (`self.IsInspecting`)
      (if (`self.IsRotatingInspect`)
        (`/Engine/EditorBlueprintResources/StandardMacros.IsValid` (`self.InspectMeshComp`)
          (:`Is Valid`
            (bind _output_get (set `self.InspectYaw` (+ (* (* _x (`self.RotationSpeed`)) -1.0) (`self.InspectYaw`))))
            (bind _output_get_2 (set `self.InspectPitch` (`KismetMathLibrary.FClamp` (+ (* (* _y (`self.RotationSpeed`)) 1.0) (`self.InspectPitch`)) -80.0 80.0)))
            (`SceneComponent.K2_SetRelativeRotation` (`self.InspectYawPivot`) (`KismetMathLibrary.MakeRotator` 0.0 0.0 _output_get) false false)
            (`SceneComponent.K2_SetRelativeRotation` (`self.InspectPitchPivot`) (`KismetMathLibrary.MakeRotator` 0.0 _output_get_2) false false)
            (`KismetSystemLibrary.PrintString` (`KismetTextLibrary.Conv_TextToString` (`|FormatText` "YawPivotYaw={YawA} | PitchPivotYaw={YawB}" (.yaw (`SceneComponent.K2_GetComponentRotation` (`self.InspectYawPivot`))) (.pitch (`SceneComponent.K2_GetComponentRotation` (`self.InspectPitchPivot`))))) true false (struct :`G` 0.66 :`B` 1.0 :`A` 1.0) 0.1)
            (set `self.LastTouchPos` _returnvalue_2))))
      (elif (`self.IsRightSide`)
        (bind _output_get_3 (set `self.TouchCurrentLocation` _returnvalue))
        (bind (_x_2 _y_2) (`KismetMathLibrary.BreakVector2D` (- _output_get_3 (`self.TouchStartLocation`))))
        (`self.AddControllerYawInput` (* _x_2 (`self.SensX`)))
        (`self.AddControllerPitchInput` (* _y_2 (`self.SensY`)))
        (set `self.TouchStartLocation` (`self.TouchCurrentLocation`))
        (else
          (`KismetSystemLibrary.PrintString` "Left Side"))))))

(fn `Aim`
  (params (`X Axis` :type "Float (double-precision)") (`Y Axis` :type "Float (double-precision)"))
  (if (not (`self.Frozen`))
    (`self.AddControllerYawInput` `X Axis`)
    (bind _result (`/Engine/EditorBlueprintResources/StandardMacros.NegateFloat` `Y Axis`)
      (:`  `
        (`self.AddControllerPitchInput` _result)))))

(fn `Freeze`
  (set `self.Frozen` true))

(fn `Hide`
  ; Missing the component to disable its collisions
  (`self.Freeze`)
  (`self.SetActorHiddenInGame` true)
  (set `self.Hidden` true)
  (set `/Game/Blueprints/Player/BP_PlayerController.IsHiding` true (`/Game/Blueprints/BPFL_Library.GetController`))
  (`PrimitiveComponent.SetCollisionEnabled` (`self.Mesh`) "NoCollision"))

(fn `Move`
  (params (`X Axis` :type "Float (double-precision)") (`Y Axis` :type "Float (double-precision)"))
  (bind (_returnvalue_roll _returnvalue_pitch _returnvalue_yaw) (`KismetMathLibrary.BreakRotator` (`self.GetControlRotation`)))
  (bind (_returnvalue_roll_2 _returnvalue_pitch_2 _returnvalue_yaw_2) (`KismetMathLibrary.BreakRotator` (`self.GetControlRotation`)))
  (if (not (`self.Frozen`))
    (`self.AddMovementInput` (`KismetMathLibrary.GetRightVector` (`KismetMathLibrary.MakeRotator` _returnvalue_roll_2 0.0 _returnvalue_yaw_2)) `X Axis`)
    (`self.AddMovementInput` (`KismetMathLibrary.GetForwardVector` (`KismetMathLibrary.MakeRotator` 0.0 0.0 _returnvalue_yaw)) `Y Axis`)))

(fn `StartInspectItem`
  (params (MeshToInspect :type "StaticMesh Object Reference"))
  (bind _returnvalue (`GameplayStatics.GetPlayerController` 0))
  (bind _returnvalue_2 (`|SpawnActorFromClass` "/Game/Blueprints/Player/Inventory/BP_InspectItem.BP_InspectItem_C" (`SceneComponent.K2_GetComponentToWorld` (`self.InspectPitchPivot`)) "AlwaysSpawn" "OverrideRootScale" (`GameplayStatics.GetPlayerController` 0) null))
  (bind _output_get (set `self.InspectActor` _returnvalue_2))
  (`self.K2_AttachToComponent` _output_get (`self.InspectPitchPivot`) "None" "SnapToTarget" "SnapToTarget" "KeepWorld" true)
  (bind _asbp_inspect_item (cast `/Game/Blueprints/Player/Inventory/BP_InspectItem` (`self.InspectActor`)))
  (bind _output_get_2 (set `self.InspectMeshComp` (`/Game/Blueprints/Player/Inventory/BP_InspectItem.ItemMesh` _asbp_inspect_item)))
  (`KismetSystemLibrary.PrintString` "Cast reussi")
  (`StaticMeshComponent.SetStaticMesh` _output_get_2 "/Game/Developers/Marwan/Meshes/Gameplay/SM_Key_001.SM_Key_001")
  (set `self.IsInspecting` true)
  (bind _output_get_3 (set `self.InspectYaw` 0.0))
  (bind _output_get_4 (set `self.InspectPitch` 0.0))
  (bind _returnvalue_3 (`KismetMathLibrary.MakeRotator` 0.0 _output_get_4 _output_get_3))
  (`SceneComponent.K2_SetRelativeRotation` (`self.InspectYawPivot`) _returnvalue_3 false false)
  (`SceneComponent.K2_SetRelativeRotation` (`self.InspectPitchPivot`) _returnvalue_3 false false)
  (set `self.IsInspecting` true)
  (set `self.IsRotatingInspect` false)
  (`Controller.SetIgnoreMoveInput` _returnvalue true)
  (`Controller.SetIgnoreLookInput` _returnvalue true)
  (set `PlayerController.bShowMouseCursor` true _returnvalue)
  (`KismetSystemLibrary.PrintString` "Enter Inspect"))

(fn `StopInspectItem`
  (bind _returnvalue (`GameplayStatics.GetPlayerController` 0))
  (`KismetSystemLibrary.PrintString` "StopInspectCalled")
  (set `self.IsRotatingInspect` false)
  (set `self.IsInspecting` false)
  (`/Engine/EditorBlueprintResources/StandardMacros.IsValid` (`self.InspectActor`)
    (:`Is Valid`
      (`self.K2_DestroyActor` (`self.InspectActor`))
      (set `self.InspectActor` null)
      (set `self.InspectMeshComp` null)
      (`Controller.SetIgnoreLookInput` _returnvalue false)
      (`Controller.SetIgnoreMoveInput` _returnvalue false)
      (`KismetSystemLibrary.PrintString` "Look Enabled")
      (set `PlayerController.bShowMouseCursor` true _returnvalue)
      (`WidgetBlueprintLibrary.SetInputMode_GameOnly` _returnvalue))))

(fn `Unfreeze`
  (set `self.Frozen` false))

(fn `Unhide`
  ; Missing the component to disable its collisions
  (`self.Unfreeze`)
  (`self.SetActorHiddenInGame` false)
  (set `self.Hidden` false)
  (set `/Game/Blueprints/Player/BP_PlayerController.IsHiding` false (`/Game/Blueprints/BPFL_Library.GetController`))
  (`PrimitiveComponent.SetCollisionEnabled` (`self.Mesh`) "QueryAndPhysics"))

(fn `UserConstructionScript`)