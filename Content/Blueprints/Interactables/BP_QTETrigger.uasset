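; BP_QTETrigger is an interactable that starts a quick time event when the player interacts with it.
; After the parent Interact logic, it freezes the player and switches the main UI to the QTE UI.
; It then passes its QTEToTrigger and itself as initiator to the QTEManager's widget, which starts the event.
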(fn `Interact`
  (bind _qtewidget (`/Game/Blueprints/BP_QTE_Manager.QTEWidget` (`self.QTEManager`)))
  (`parent.Interact`)
  (`/Game/Blueprints/Player/BP_Player.Freeze` (`/Game/Blueprints/BPFL_Library.GetPlayer`))
  (`/Game/Blueprints/UI/WBP_MainUI.SwitchToQTEUI` (`/Game/Blueprints/Player/BP_PlayerController.MainUI` (`/Game/Blueprints/BPFL_Library.GetController`)))
  (`/Game/Blueprints/UI/WBP_QTEUI.SetNewQTEToPlay` _qtewidget (`self.QTEToTrigger`) self)
  (`/Game/Blueprints/UI/WBP_QTEUI.StartNextQTE` _qtewidget true))

(fn `UserConstructionScript`
  (`parent.UserConstructionScript`))