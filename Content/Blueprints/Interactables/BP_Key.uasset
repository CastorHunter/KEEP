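; BP_Key is a pickup key interactable that grants its key type to the player on interaction.
; It marks itself interactable on BeginPlay.
; Interacting runs the parent logic, adds KeyType to the controller's Keys and the key itself to its Items, then destroys the actor.
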(event `self.ReceiveBeginPlay`
  (set `self.Interactable` true))

(fn `Interact`
  (bind _playercontroller (`/Game/Blueprints/BPFL_Library.GetController`))
  (`parent.Interact`)
  (`KismetArrayLibrary.Array_Add` (`/Game/Blueprints/Player/BP_PlayerController.Keys` _playercontroller) (`self.KeyType`))
  (`KismetArrayLibrary.Array_Add` (`/Game/Blueprints/Player/BP_PlayerController.Items` _playercontroller) self)
  (`self.K2_DestroyActor`))

(fn `UserConstructionScript`
  (`parent.UserConstructionScript`))