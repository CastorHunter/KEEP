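; BP_Closet is an interactable closet the player hides in, with a quick time event on interaction.
; Interact freezes the player, switches to QTE UI and starts the closet's assigned QTE with itself as initiator.
; HidePlayerInThisCloset unfreezes and hides the player, blends the view to the closet, shows closet UI and starts stressing.
; Show and hide interactable overrides toggle the mesh's custom depth stencil value.
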(event `self.ReceiveBeginPlay`
  (set `self.Interactable` true))

(fn `HideInteractable`
  (`parent.HideInteractable`)
  (`PrimitiveComponent.SetCustomDepthStencilValue` (`self.Mesh`) 0))

(fn `HidePlayerInThisCloset`
  (bind _player (`/Game/Blueprints/BPFL_Library.GetPlayer`))
  (bind _playercontroller (`/Game/Blueprints/BPFL_Library.GetController`))
  (`/Game/Blueprints/Player/BP_Player.Unfreeze` _player)
  (`/Game/Blueprints/Player/BP_Player.Hide` _player)
  (`PlayerController.SetViewTargetWithBlend` (`/Game/Blueprints/BPFL_Library.GetController`) self 0.0 "VTBlend_Cubic" 0.0 false)
  (`/Game/Blueprints/UI/WBP_MainUI.SwitchToClosetUI` (`/Game/Blueprints/Player/BP_PlayerController.MainUI` _playercontroller))
  (`/Game/Blueprints/Player/BP_PlayerController.StartStressing` _playercontroller))

(fn `Interact`
  (bind _qtewidget (`/Game/Blueprints/BP_QTE_Manager.QTEWidget` (`/Game/Blueprints/Player/BP_PlayerController.QTEManager` (`/Game/Blueprints/BPFL_Library.GetController`))))
  (`parent.Interact`)
  (`/Game/Blueprints/Player/BP_Player.Freeze` (`/Game/Blueprints/BPFL_Library.GetPlayer`))
  (`/Game/Blueprints/UI/WBP_MainUI.SwitchToQTEUI` (`/Game/Blueprints/Player/BP_PlayerController.MainUI` (`/Game/Blueprints/BPFL_Library.GetController`)))
  (`/Game/Blueprints/UI/WBP_QTEUI.SetNewQTEToPlay` _qtewidget (`self.QTEToTrigger`) self)
  (`/Game/Blueprints/UI/WBP_QTEUI.StartNextQTE` _qtewidget true))

(fn `ShowInteractable`
  (`parent.ShowInteractable`)
  (`PrimitiveComponent.SetCustomDepthStencilValue` (`self.Mesh`) 1))

(fn `UserConstructionScript`
  (`parent.UserConstructionScript`))