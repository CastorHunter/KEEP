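; BP_Letter is a readable letter that the player can interact with, extending a parent interactable's behaviour.
; It marks itself interactable on BeginPlay, and its show and hide overrides toggle the Cube mesh's custom depth stencil value after calling the parent.
; Interacting runs the parent logic, freezes the player, then calls ReadLetter on the controller's PlayerUI.
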(event `self.ReceiveBeginPlay`
  (set `self.Interactable` true))

(fn `HideInteractable`
  (`parent.HideInteractable`)
  (`PrimitiveComponent.SetCustomDepthStencilValue` (`self.Cube`) 0))

(fn `Interact`
  (`parent.Interact`)
  (`/Game/Blueprints/Player/BP_Player.Freeze` (`/Game/Blueprints/BPFL_Library.GetPlayer`))
  (`/Game/Blueprints/UI/WBP_PlayerUI.Read Letter` (`/Game/Blueprints/Player/BP_PlayerController.PlayerUI` (`/Game/Blueprints/BPFL_Library.GetController`)) null))

(fn `ShowInteractable`
  (`parent.ShowInteractable`)
  (`PrimitiveComponent.SetCustomDepthStencilValue` (`self.Cube`) 1))

(fn `UserConstructionScript`
  (`parent.UserConstructionScript`))