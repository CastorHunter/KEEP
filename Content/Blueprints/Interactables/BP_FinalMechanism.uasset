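; Final mechanism interactable that requires two specific items among the controller's keys and opens the last door.
; With both items held, Interact freezes the player, switches to the QTE UI and starts a quick-time event with itself as initiator.
; OpenLastDoor, marked temporary, opens the door, restores player control and UI, disables interaction, plays a sound and swaps the mesh.
; Custom depth stencil values toggle the interactable highlight.
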(event `self.ReceiveBeginPlay`
  (set `self.Interactable` true))

(fn `HideInteractable`
  (`parent.HideInteractable`)
  (`PrimitiveComponent.SetCustomDepthStencilValue` (`self.Cube`) 0))

(fn `Interact`
  (bind _qtewidget (`/Game/Blueprints/BP_QTE_Manager.QTEWidget` (`/Game/Blueprints/Player/BP_PlayerController.QTEManager` (`/Game/Blueprints/BPFL_Library.GetController`))))
  (`parent.Interact`)
  (for _array_element (`/Game/Blueprints/Player/BP_PlayerController.Keys` (`/Game/Blueprints/BPFL_Library.GetController`))
    (if (`|EnumEquality` _array_element (`self.ItemNeeded`))
      (for _array_element_2 (`/Game/Blueprints/Player/BP_PlayerController.Keys` (`/Game/Blueprints/BPFL_Library.GetController`))
        (if (`|EnumEquality` _array_element_2 (`self.SecondItemNeeded`))
          (`/Game/Blueprints/Player/BP_Player.Freeze` (`/Game/Blueprints/BPFL_Library.GetPlayer`))
          (`/Game/Blueprints/UI/WBP_MainUI.SwitchToQTEUI` (`/Game/Blueprints/Player/BP_PlayerController.MainUI` (`/Game/Blueprints/BPFL_Library.GetController`)))
          (`/Game/Blueprints/UI/WBP_QTEUI.SetNewQTEToPlay` _qtewidget "NewEnumerator3" self)
          (`/Game/Blueprints/UI/WBP_QTEUI.StartNextQTE` _qtewidget true))))))

(fn `OpenLastDoor`
  ; Temporary
  (`/Game/Blueprints/BP_FinalDoor.OpenFinalDoor` (`self.LastDoor`))
  (`/Game/Blueprints/UI/WBP_MainUI.SwitchToPlayerUI` (`/Game/Blueprints/Player/BP_PlayerController.MainUI` (`/Game/Blueprints/BPFL_Library.GetController`)))
  (`/Game/Blueprints/Player/BP_Player.Unfreeze` (`/Game/Blueprints/BPFL_Library.GetPlayer`))
  (set `self.Interactable` false)
  (`GameplayStatics.PlaySoundAtLocation` "/Game/Sound/OpeningHarrow.OpeningHarrow" (`self.K2_GetActorLocation`) (struct) 1.0 1.0 0.0 null null null null)
  (`StaticMeshComponent.SetStaticMesh` (`self.Cube`) "/Game/Meshes/Gameplay/SM_MechanismRope_001.SM_MechanismRope_001"))

(fn `ShowInteractable`
  (`parent.ShowInteractable`)
  (`PrimitiveComponent.SetCustomDepthStencilValue` (`self.Cube`) 1))

(fn `UserConstructionScript`
  (`parent.UserConstructionScript`))