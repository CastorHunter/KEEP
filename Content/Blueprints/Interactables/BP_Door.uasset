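; Interactable door that gates opening behind a required key and a quick time event (QTE).
; Interact scans the controller's Keys for KeyNeeded and, on a match, freezes the player, switches to the QTE UI and starts a QTE with the door as initiator.
; OpenDoor, not called within this Blueprint, disables interaction, snaps the door's yaw by 90 degrees, restores the player UI and unfreezes the player.
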(event `self.ReceiveBeginPlay`
  (set `self.Interactable` true))

(fn `Interact`
  (bind _qtewidget (`/Game/Blueprints/BP_QTE_Manager.QTEWidget` (`/Game/Blueprints/Player/BP_PlayerController.QTEManager` (`/Game/Blueprints/BPFL_Library.GetController`))))
  (`parent.Interact`)
  (for _array_element (`/Game/Blueprints/Player/BP_PlayerController.Keys` (`/Game/Blueprints/BPFL_Library.GetController`))
    (if (`|EnumEquality` _array_element (`self.KeyNeeded`))
      (`/Game/Blueprints/Player/BP_Player.Freeze` (`/Game/Blueprints/BPFL_Library.GetPlayer`))
      (`/Game/Blueprints/UI/WBP_MainUI.SwitchToQTEUI` (`/Game/Blueprints/Player/BP_PlayerController.MainUI` (`/Game/Blueprints/BPFL_Library.GetController`)))
      (`/Game/Blueprints/UI/WBP_QTEUI.SetNewQTEToPlay` _qtewidget "NewEnumerator2" self)
      (`/Game/Blueprints/UI/WBP_QTEUI.StartNextQTE` _qtewidget true))))

(fn `OpenDoor`
  (bind (_returnvalue_roll _returnvalue_pitch _returnvalue_yaw) (`KismetMathLibrary.BreakRotator` (`self.K2_GetActorRotation`)))
  (set `self.Interactable` false)
  (`self.K2_SetActorRotation` (`KismetMathLibrary.MakeRotator` _returnvalue_roll _returnvalue_pitch (+ _returnvalue_yaw 90.0)))
  (`/Game/Blueprints/UI/WBP_MainUI.SwitchToPlayerUI` (`/Game/Blueprints/Player/BP_PlayerController.MainUI` (`/Game/Blueprints/BPFL_Library.GetController`)))
  (`/Game/Blueprints/Player/BP_Player.Unfreeze` (`/Game/Blueprints/BPFL_Library.GetPlayer`)))

(fn `UserConstructionScript`
  (`parent.UserConstructionScript`))