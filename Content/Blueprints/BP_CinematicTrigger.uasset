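; Trigger actor that plays one of two in-game cinematics on overlap, selected by CinematicToPlay.
; It freezes the player and blends the view to itself, then plays montages for either a walking enemy or the player's escape with an enemy death.
; The walking branch waits, then destroys the enemy and trigger.
; Both branches unfreeze the player and restore the camera, the escape one immediately after starting its montages.
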(event `self.ReceiveActorBeginOverlap`
  (params (OtherActor :type "Actor Object Reference"))
  (bind _enemywalking (`self.EnemyWalking`))
  (`/Game/Blueprints/Player/BP_Player.Freeze` (`/Game/Blueprints/BPFL_Library.GetPlayer`))
  (`PlayerController.SetViewTargetWithBlend` (`/Game/Blueprints/BPFL_Library.GetController`) self 1.5 "VTBlend_Cubic" 0.0 false)
  (switch `/Game/Enums/E_CinematicType` (`self.CinematicToPlay`)
    (:`NewEnumerator1`
      (`Character.PlayAnimMontage` _enemywalking "/Game/Animation/AM_EnemyWalking.AM_EnemyWalking" 1.0 "None")
      (`KismetSystemLibrary.Delay` 7.0)
      (`self.K2_DestroyActor` _enemywalking)
      (`self.K2_DestroyActor`))
    (:`NewEnumerator2`
      (`Character.PlayAnimMontage` (`/Game/Blueprints/BPFL_Library.GetPlayer`) "/Game/Animation/AM_PlayerEscaping.AM_PlayerEscaping" 1.0 "None")
      (`Character.PlayAnimMontage` (`/Game/Blueprints/Player/BP_PlayerController.EnemyReference` (`/Game/Blueprints/BPFL_Library.GetController`)) "/Game/Animation/AM_EnemyDeath.AM_EnemyDeath" 1.0 "None")))
  (`/Game/Blueprints/Player/BP_Player.Unfreeze` (`/Game/Blueprints/BPFL_Library.GetPlayer`))
  (`PlayerController.SetViewTargetWithBlend` (`/Game/Blueprints/BPFL_Library.GetController`) (`/Game/Blueprints/BPFL_Library.GetPlayer`) 0.0 "VTBlend_Cubic" 0.0 false))

(fn `UserConstructionScript`)