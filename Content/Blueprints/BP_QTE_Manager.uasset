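; Quick-time event manager that registers with the controller and judges Tap, DoubleTap, Hold, Slash and Slide gestures.
; Off mobile, it samples mouse viewport positions for press, release and current pointer.
; Each gesture polls these against targets and precision in timeline updates, chaining timelines for multi-step gestures.
; Successes advance the QTE widget; timeouts report failure except Tap, and DoubleTap's between-tap timing is marked unfinished.
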(event `self.ReceiveBeginPlay`
  (bind _playercontroller (`/Game/Blueprints/BPFL_Library.GetController`))
  (set `/Game/Blueprints/Player/BP_PlayerController.QTEManager` self _playercontroller)
  (`KismetSystemLibrary.Delay` 1.0)
  (set `self.QTEWidget` (`/Game/Blueprints/Player/BP_PlayerController.QTEUI` _playercontroller)))

(event `Set Pressed Position`
  ; For Computer
  (if (not (`/Game/Blueprints/BPFL_Library.GetOnMobile`))
    (bind _returnvalue (`WidgetLayoutLibrary.GetMousePositionOnViewport`))
    (set `self.PressedPosition` (`KismetMathLibrary.MakeVector` (`KismetMathLibrary.BreakVector2D` _returnvalue) (`.Y` (`KismetMathLibrary.BreakVector2D` _returnvalue))))))

(event `Key|H`
  (params (Key :type "Key Structure"))
  (:`Pressed`
    (`KismetSystemLibrary.PrintString` (`KismetStringLibrary.Conv_VectorToString` (`self.ReleasedPosition`)))))

(event `Set Released Position`
  ; For Computer
  (if (not (`/Game/Blueprints/BPFL_Library.GetOnMobile`))
    (bind _returnvalue (`WidgetLayoutLibrary.GetMousePositionOnViewport`))
    (set `self.ReleasedPosition` (`KismetMathLibrary.MakeVector` (`KismetMathLibrary.BreakVector2D` _returnvalue) (`.Y` (`KismetMathLibrary.BreakVector2D` _returnvalue))))))

(event `Key|N`
  (params (Key :type "Key Structure"))
  (:`Pressed`
    (`KismetSystemLibrary.PrintString` (`KismetStringLibrary.Conv_DoubleToString` (`TimelineComponent.GetPlaybackPosition` (`self.TapTimeline`))))))

(event `self.ReceiveTick`
  (params (DeltaSeconds :type "Float (single-precision)"))
  ; For Computer
  (if (not (`/Game/Blueprints/BPFL_Library.GetOnMobile`))
    (bind _returnvalue (`WidgetLayoutLibrary.GetMousePositionOnViewport`))
    (set `self.ActualPosition` (`KismetMathLibrary.MakeVector` (`KismetMathLibrary.BreakVector2D` _returnvalue) (`.Y` (`KismetMathLibrary.BreakVector2D` _returnvalue))))))

(event `Tap`
  (params (Position :type "Vector Structure") (Precision :type "Float (double-precision)") (TimeToDo :type "Float (double-precision)"))
  (bind _pressedposition (`self.PressedPosition`))
  (`TimelineComponent.SetPlayRate` (`self.TapTimeline`) (/ 1.0 TimeToDo))
  (set `self.QTE_Enabled` true)
  (`Timeline|TapTimeline` :!via `PlayFromStart` :!label _label
    (:`Update`
      (if (and (!= (`self.ReleasedPosition`) (0.0 0.0 0.0)) (!= _pressedposition (0.0 0.0 0.0)))
        (if (== _pressedposition Position :`ErrorTolerance` Precision)
          (set `self.QTE_Enabled` false)
          (`|ExecutionSequence`
            (:`then_0`
              (goto _label :!via `Stop`))
            (:`then_1`
              (`/Game/Blueprints/UI/WBP_QTEUI.StartNextQTE` (`self.QTEWidget`) true))))))
    (:`Finished`
      (set `self.QTE_Enabled` false))))

(event `DoubleTap`
  (params (Position :type "Vector Structure") (Precision :type "Float (double-precision)") (TimeBetweenTaps :type "Float (double-precision)") (TimeToDo :type "Float (double-precision)"))
  (bind _pressedposition (`self.PressedPosition`))
  (bind _pressedposition_2 (`self.PressedPosition`))
  ; Time between Taps does not work yet
  (`TimelineComponent.SetPlayRate` (`self.FirstTapTimeline`) (/ 1.0 TimeToDo))
  (set `self.QTE_Enabled` true)
  (`Timeline|FirstTapTimeline` :!via `PlayFromStart` :!label _label_2
    (:`Update`
      (if (and (!= (`self.ReleasedPosition`) (0.0 0.0 0.0)) (!= _pressedposition (0.0 0.0 0.0)))
        (if (== _pressedposition Position :`ErrorTolerance` Precision)
          (`Timeline|SecondTapTimeline` :!via `PlayFromStart` :!label _label_3
            (:`Update`
              (if (and (!= (`self.ReleasedPosition`) (0.0 0.0 0.0)) (!= _pressedposition_2 (0.0 0.0 0.0)))
                (if (== _pressedposition_2 Position :`ErrorTolerance` Precision)
                  (set `self.QTE_Enabled` false)
                  (`|ExecutionSequence`
                    (:`then_0`
                      (`|ExecutionSequence`
                        (:`then_0`
                          (goto _label_2 :!via `Stop`))
                        (:`then_1`
                          (goto _label_3 :!via `Stop`))))
                    (:`then_1`
                      (`/Game/Blueprints/UI/WBP_QTEUI.StartNextQTE` (`self.QTEWidget`) true))))))))))
    (:`Finished`
      (set `self.QTE_Enabled` false)
      (`/Game/Blueprints/UI/WBP_QTEUI.StartNextQTE` (`self.QTEWidget`) false))))

(event `Hold`
  (params (Position :type "Vector Structure") (Precision :type "Float (double-precision)") (TimeToHold :type "Float (double-precision)") (TimeToDo :type "Float (double-precision)"))
  (bind _pressedposition (`self.PressedPosition`))
  (bind _releasedposition (`self.ReleasedPosition`))
  (`TimelineComponent.SetPlayRate` (`self.FirstPressionTimeline`) (/ 1.0 TimeToDo))
  (set `self.QTE_Enabled` true)
  (`Timeline|FirstPressionTimeline` :!via `PlayFromStart` :!label _label_4
    (:`Update`
      (if (!= _pressedposition (0.0 0.0 0.0))
        (if (== _pressedposition Position :`ErrorTolerance` Precision)
          (`KismetSystemLibrary.Delay` TimeToHold)
          (`Timeline|Timeline_0` :!via `PlayFromStart` :!label _label_5
            (:`Update`
              (if (and (!= _releasedposition (0.0 0.0 0.0)) (== _releasedposition (`self.PressedPosition`) :`ErrorTolerance` 20.0))
                (if (== _releasedposition Position :`ErrorTolerance` Precision)
                  (set `self.QTE_Enabled` false)
                  (`|ExecutionSequence`
                    (:`then_0`
                      (`|ExecutionSequence`
                        (:`then_0`
                          (goto _label_4 :!via `Stop`))
                        (:`then_1`
                          (goto _label_5 :!via `Stop`))))
                    (:`then_1`
                      (`/Game/Blueprints/UI/WBP_QTEUI.StartNextQTE` (`self.QTEWidget`) true))))))))))
    (:`Finished`
      (set `self.QTE_Enabled` false)
      (`/Game/Blueprints/UI/WBP_QTEUI.StartNextQTE` (`self.QTEWidget`) false))))

(event `Slash`
  (params (Direction :type "EDirection Enum" :default "Left") (Target :type "Vector Structure") (Precision :type "Float (double-precision)") (TimeToDo :type "Float (double-precision)"))
  (bind (_pressedposition_x _pressedposition_y) (`KismetMathLibrary.BreakVector` (`self.PressedPosition`)))
  (bind (_releasedposition_x _releasedposition_y) (`KismetMathLibrary.BreakVector` (`self.ReleasedPosition`)))
  (bind _returnvalue (> _pressedposition_y _releasedposition_y))
  (bind _returnvalue_2 (> _pressedposition_x _releasedposition_x))
  (bind _returnvalue_3 (and (and (!= _pressedposition_y 0.0) (!= _releasedposition_y 0.0)) (and (!= _pressedposition_x 0.0) (!= _releasedposition_x 0.0))))
  (`self.ClearQTE`)
  (set `self.ReleasedPosition` (0.0 0.0 0.0))
  (set `self.PressedPosition` (0.0 0.0 0.0))
  (`TimelineComponent.SetPlayRate` (`self.FirstPressionTimeline`) (/ 1.0 TimeToDo))
  (set `self.QTE_Enabled` true)
  (`Timeline|SlashTimeline` :!via `PlayFromStart` :!label _label_6
    (:`Update`
      (if (== (`self.ActualPosition`) Target :`ErrorTolerance` Precision)
        (switch `EDirection` Direction
          (:`Left`
            (if (and _returnvalue_2 _returnvalue_3)
              (set `self.QTE_Enabled` false :!label _label_7)
              (`|ExecutionSequence`
                (:`then_0`
                  (goto _label_6 :!via `Stop`))
                (:`then_1`
                  (`/Game/Blueprints/UI/WBP_QTEUI.StartNextQTE` (`self.QTEWidget`) true)))))
          (:`Right`
            (if (and (not _returnvalue_2) _returnvalue_3)
              (`KismetSystemLibrary.PrintString` (`KismetStringLibrary.Conv_DoubleToString` _pressedposition_x))
              (`KismetSystemLibrary.PrintString` (`KismetStringLibrary.Conv_DoubleToString` _releasedposition_x))
              (goto _label_7)))
          (:`Up`
            (if (and _returnvalue _returnvalue_3)
              (goto _label_7)))
          (:`Down`
            (if (and (not _returnvalue) _returnvalue_3)
              (goto _label_7))))))
    (:`Finished`
      (set `self.QTE_Enabled` false)
      (`/Game/Blueprints/UI/WBP_QTEUI.StartNextQTE` (`self.QTEWidget`) false))))

(event `Slide`
  (params (StartPosition :type "Vector Structure") (EndPosistion :type "Vector Structure") (Precision :type "Float (double-precision)") (TimeToDo :type "Float (double-precision)"))
  (bind _pressedposition (`self.PressedPosition`))
  (bind _releasedposition (`self.ReleasedPosition`))
  (`TimelineComponent.SetPlayRate` (`self.FirstPressionTimeline`) (/ 1.0 0.0))
  (set `self.QTE_Enabled` true)
  (`Timeline|SlideTimelinePressed` :!via `PlayFromStart` :!label _label_8
    (:`Update`
      (if (!= _pressedposition (0.0 0.0 0.0))
        (if (== _pressedposition StartPosition :`ErrorTolerance` Precision)
          (`Timeline|SlideTimelineReleased` :!via `PlayFromStart` :!label _label_9
            (:`Update`
              (if (!= _releasedposition (0.0 0.0 0.0))
                (if (== _releasedposition EndPosistion :`ErrorTolerance` Precision)
                  (set `self.QTE_Enabled` false)
                  (`|ExecutionSequence`
                    (:`then_0`
                      (`|ExecutionSequence`
                        (:`then_0`
                          (goto _label_8 :!via `Stop`))
                        (:`then_1`
                          (goto _label_9 :!via `Stop`))))
                    (:`then_1`
                      (`/Game/Blueprints/UI/WBP_QTEUI.StartNextQTE` (`self.QTEWidget`) true))))))))))
    (:`Finished`
      (set `self.QTE_Enabled` false)
      (`/Game/Blueprints/UI/WBP_QTEUI.StartNextQTE` (`self.QTEWidget`) false))))

(event `ClearQTE`
  (set `self.ReleasedPosition` (0.0 0.0 0.0))
  (set `self.ActualPosition` (0.0 0.0 0.0))
  (set `self.PressedPosition` (0.0 0.0 0.0)))

(fn `UserConstructionScript`)