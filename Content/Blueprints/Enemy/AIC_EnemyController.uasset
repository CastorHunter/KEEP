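; AI controller for enemies that detect, attack, investigate and seek using sight and hearing.
; On possess it runs BT_EnemyBehavior and writes an E_EnemyStates value, target and point of interest to the blackboard.
; Perception updates drive transitions: sight attacks a visible player, hearing investigates, lost sight seeks.
; A looping timer handles forgotten actors, while a Tick marked for removal polls player hiding to drop or start attacks.
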(event `self.ReceivePossess`
  (params (PossessedPawn :type "Pawn Object Reference"))
  (bind _blackboardcomponent (`self.UseBlackboard` "/Game/AI/BB_EnemyBehavior.BB_EnemyBehavior"))
  (set `self.Blackboard Component` _blackboardcomponent)
  (`self.RunBehaviorTree` "/Game/AI/BT_EnemyBehavior.BT_EnemyBehavior")
  (`self.SetStateAsPassive`)
  (bind _returnvalue (`KismetSystemLibrary.K2_SetTimerDelegate` (`|CreateDelegate` :!event `CheckIfSeenActors`) 0.5 true))
  (set `self.CheckForgottenActorsTimer` _returnvalue))

(event `self.ReceiveUnPossess`
  (params (UnpossessedPawn :type "Pawn Object Reference"))
  (`KismetSystemLibrary.K2_ClearAndInvalidateTimerHandle` (`self.CheckForgottenActorsTimer`)))

(event `self.AIPerception.OnPerceptionUpdated`
  (params (UpdatedActors :type "Array of Actor Object Reference (by ref)"))
  (for _array_element UpdatedActors
    (`|ExecutionSequence`
      (:`then_0`
        (if (`self.CanSenseActor` _array_element "NewEnumerator1")
          (`self.HandleSenseSight` _array_element)
          (else
            (`self.HandleLostSight` _array_element))))
      (:`then_1`
        (bind (_sensed _stimulus) (`self.CanSenseActor` _array_element "NewEnumerator2"))
        (if _sensed
          (`self.HandleSenseHearing` (`.StimulusLocation` (break `AIStimulus` _stimulus))))))))

(event `CheckIfSeenActors`
  (if (!= (`KismetArrayLibrary.Array_Length` (`self.KnownSeenActors`)) (`KismetArrayLibrary.Array_Length` (`AIPerceptionComponent.GetKnownPerceivedActors` (`self.AIPerception`) null)))
    (for _array_element (`self.KnownSeenActors`)
      (if (== (`KismetArrayLibrary.Array_Find` (`AIPerceptionComponent.GetKnownPerceivedActors` (`self.AIPerception`) null) _array_element) -1)
        (`self.HandleForgotActors` _array_element)))))

(event `self.ReceiveTick`
  (params (DeltaSeconds :type "Float (single-precision)"))
  (bind _attacktarget (`self.AttackTarget`))
  ; To Remove (tick to disable)
  (`self.SetPlayerIsHiding`)
  (`/Engine/EditorBlueprintResources/StandardMacros.IsValid` _attacktarget
    (:`Is Valid`
      (if (== (`self.K2_GetActorLocation` (`self.K2_GetPawn`)) (`self.K2_GetActorLocation` _attacktarget) :`ErrorTolerance` 1.0)
        (set `self.AttackTarget` null)))))

(fn `CanSenseActor`
  (params (Actor :type "Actor Object Reference") (Sense :type "/Game/Enums/E_AISenses Enum" :default "NewEnumerator0"))
  (returns (Sensed :type Boolean) (Stimulus :type "AIStimulus Structure"))
  (bind _info (`AIPerceptionComponent.GetActorsPerception` (`self.AIPerception`) Actor))
  (for _array_element (`.LastSensedStimuli` (break `ActorPerceptionBlueprintInfo` _info))
    (bind _returnvalue (`AIPerceptionSystem.GetSenseClassForStimulus` _array_element))
    (if (== _returnvalue (select `/Game/Enums/E_AISenses` Sense :`NewEnumerator1` "/Script/AIModule.AISense_Sight" :`NewEnumerator2` "/Script/AIModule.AISense_Hearing" :!type "Object Class Reference"))
      (return (`.bSuccessfullySensed` (break `AIStimulus` _array_element)) _array_element))))

(fn `GetCurrentState`
  (returns (State :type "/Game/Enums/E_EnemyStates Enum"))
  (return (cast `/Game/Enums/E_EnemyStates` (`BlackboardComponent.GetValueAsEnum` (`self.Blackboard`) (`self.StateKeyName`)))))

(fn `HandleForgotActors`
  (params (Actor :type "Actor Object Reference"))
  (`KismetArrayLibrary.Array_RemoveItem` (`self.KnownSeenActors`) Actor)
  (if (== Actor (`self.AttackTarget`))
    (`self.SetStateAsPassive`)))

(fn `HandleLostSight`
  (params (Actor :type "Actor Object Reference"))
  (if (== Actor (`self.AttackTarget`))
    (bind _state (`self.GetCurrentState`))
    (switch `/Game/Enums/E_EnemyStates` _state
      (:`NewEnumerator1`
        _)
      (:`NewEnumerator2`
        _)
      (:`NewEnumerator4`
        _))
    (`self.SetStateAsSeeking` (`self.K2_GetActorLocation` (`self.AttackTarget`)))))

(fn `HandleSenseHearing`
  (params (Location :type "Vector Structure"))
  (bind _state (`self.GetCurrentState`))
  (switch `/Game/Enums/E_EnemyStates` _state
    (:`NewEnumerator0`
      _)
    (:`NewEnumerator4`
      _))
  (`self.SetStateAsInvestigating` Location))

(fn `HandleSenseSight`
  (params (Actor :type "Actor Object Reference"))
  (`KismetArrayLibrary.Array_AddUnique` (`self.KnownSeenActors`))
  (bind _state (`self.GetCurrentState`))
  (switch `/Game/Enums/E_EnemyStates` _state
    (:`NewEnumerator0`
      _)
    (:`NewEnumerator3`
      _)
    (:`NewEnumerator4`
      _))
  (if (== Actor (`/Game/Blueprints/BPFL_Library.GetPlayer`))
    (if (`BlackboardComponent.GetValueAsBool` (`self.Blackboard`) (`self.PlayerIsVisibleKeyName`))
      (`self.SetStateAsAttacking` Actor)
      (else
        (`self.SetStateAsPassive`)))))

(fn `SetPlayerIsHiding`
  (bind _player (`/Game/Blueprints/BPFL_Library.GetPlayer`))
  (bind _ishiding (`/Game/Blueprints/Player/BP_PlayerController.IsHiding` (`/Game/Blueprints/BPFL_Library.GetController`)))
  (`BlackboardComponent.SetValueAsBool` (`self.Blackboard`) (`self.PlayerIsVisibleKeyName`) (not _ishiding))
  (if _ishiding
    (bind _state (`self.GetCurrentState`))
    (switch `/Game/Enums/E_EnemyStates` _state
      (:`NewEnumerator1`
        (`self.SetStateAsPassive`)))
    (elif (`self.CanSenseActor` _player)
      (`self.SetStateAsAttacking` _player))))

(fn `SetStateAsAttacking`
  (params (AttackTarget :type "Actor Object Reference"))
  (`BlackboardComponent.SetValueAsObject` (`self.Blackboard`) (`self.AttackTargetKeyName`) AttackTarget)
  (`BlackboardComponent.SetValueAsEnum` (`self.Blackboard`) (`self.StateKeyName`) (enumliteral `/Game/Enums/E_EnemyStates` "NewEnumerator1")))

(fn `SetStateAsInvestigating`
  (params (Location :type "Vector Structure"))
  (bind _blackboard (`self.Blackboard`))
  (`BlackboardComponent.SetValueAsEnum` _blackboard (`self.StateKeyName`) (enumliteral `/Game/Enums/E_EnemyStates` "NewEnumerator4"))
  (`BlackboardComponent.SetValueAsVector` _blackboard (`self.PointOfInterestKeyName`) Location))

(fn `SetStateAsPassive`
  (`BlackboardComponent.SetValueAsEnum` (`self.Blackboard`) (`self.StateKeyName`) (enumliteral `/Game/Enums/E_EnemyStates` "NewEnumerator0")))

(fn `SetStateAsSeeking`
  (params (Loaction :type "Vector Structure"))
  (bind _blackboard (`self.Blackboard`))
  (`BlackboardComponent.SetValueAsEnum` _blackboard (`self.StateKeyName`) (enumliteral `/Game/Enums/E_EnemyStates` "NewEnumerator3"))
  (`BlackboardComponent.SetValueAsVector` _blackboard (`self.PointOfInterestKeyName`) Loaction))

(fn `UserConstructionScript`)