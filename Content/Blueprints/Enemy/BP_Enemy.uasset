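; Enemy character that patrols routes and kills the player when it attacks.
; It registers with its controller on BeginPlay and syncs control rotation to actor rotation each Tick.
; Attack turns the player toward it, freezes them, then after a fixed delay has the controller kill them; the montage branch is disconnected.
; Helpers store routes in a map, pick a given or random destination, and map movement states to walk speeds.
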(event `self.ReceiveBeginPlay`
  (set `/Game/Blueprints/Player/BP_PlayerController.EnemyReference` self (`/Game/Blueprints/BPFL_Library.GetController`)))

(event `self.ReceiveTick`
  (params (DeltaSeconds :type "Float (single-precision)"))
  (`Controller.SetControlRotation` (`AIBlueprintHelperLibrary.GetAIController` self) (`self.K2_GetActorRotation` self)))

(event `Attack`
  (bind _player (`/Game/Blueprints/BPFL_Library.GetPlayer`))
  (`/Game/Blueprints/Player/BP_Player.OrientToActor` _player (`self.K2_GetActorLocation`))
  (`/Game/Blueprints/Player/BP_Player.Freeze` _player)
  (`KismetSystemLibrary.Delay` 3.0)
  (`/Engine/EditorBlueprintResources/StandardMacros.IsValid` (`/Game/Blueprints/BPFL_Library.GetPlayer`)
    (:`Is Valid`
      (`/Game/Blueprints/Player/BP_PlayerController.KillPlayer` (`/Game/Blueprints/BPFL_Library.GetController`))
      (`self.OnAttackEnd`))))

(fn `AddNewDestination`
  (params (PatrolRoute :type "/Game/Blueprints/Enemy/BP_PatrolRoute Object Reference") (PatrolRouteName :type Name))
  (`BlueprintMapLibrary.Map_Add` (`self.DestinationRoutes`) PatrolRoute PatrolRouteName))

(fn `GetPatrolRoute`
  (returns (PatrolRoute :type "/Game/Blueprints/Enemy/BP_PatrolRoute Object Reference"))
  (return (`self.PatrolRoute`)))

(fn `GetPatrolRoutes`
  (returns (PatrolRoutes :type "Array of /Game/Blueprints/Enemy/BP_PatrolRoute Object Reference"))
  (return (`self.PatrolRoutes`)))

(fn `SetMovementSpeed`
  (params (MovementSpeed :type "/Game/Enums/E_MovementSpeed Enum" :default "NewEnumerator0"))
  (returns (SpeedValue :type "Float (double-precision)"))
  (bind _output_get (set `CharacterMovementComponent.MaxWalkSpeed` (select `/Game/Enums/E_MovementSpeed` MovementSpeed :`NewEnumerator1` 150.0 :`NewEnumerator2` 300.0 :`NewEnumerator3` 500.0 :!type "Float (single-precision)") (`self.CharacterMovement`)))
  (return _output_get))

(fn `SetNewDestination`
  (params (PatrolRoute :type "/Game/Blueprints/Enemy/BP_PatrolRoute Object Reference"))
  (`/Engine/EditorBlueprintResources/StandardMacros.IsValid` PatrolRoute
    (:`Is Valid`
      (set `self.PatrolRoute` PatrolRoute))
    (:`Is Not Valid`
      (set `self.PatrolRoute` (`BlueprintMapLibrary.Map_GetKeyValueByIndex` (`self.DestinationRoutes`) (`KismetMathLibrary.RandomIntegerInRange` 0 (- (`BlueprintMapLibrary.Map_Length` (`self.DestinationRoutes`)) 1)))))))

(fn `UserConstructionScript`)